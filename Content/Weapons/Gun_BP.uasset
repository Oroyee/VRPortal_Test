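; VR gun actor that motion controllers can pick up, drop and fire.
; Pickup disables mesh physics, attaches the root to the given component and applies a fixed grip offset to the mesh, while Drop detaches and restores physics, both updating IsHeld.
; FireWeapon spawns a Bullet at the Arrow component's location, passing no rotation from the Arrow.
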(event `/Game/VirtualRealityBP/Blueprints/PickupActorInterface.Pickup`
  (params (AttachTo :type "SceneComponent Object Reference"))
  (`PrimitiveComponent.SetSimulatePhysics` (`self.StaticMeshComponent`) false)
  (`SceneComponent.K2_AttachToComponent` (`self.K2_GetRootComponent`) AttachTo "None" "SnapToTarget" "SnapToTarget" "KeepWorld" false)
  (`SceneComponent.K2_SetRelativeLocationAndRotation` (`self.StaticMeshComponent`) (2.214277 -0.02762 -2.789246) (struct :`Pitch` -0.000296 :`Yaw` -89.998055 :`Roll` 50.003963) false false)
  (set `self.IsHeld` true))

(event `/Game/VirtualRealityBP/Blueprints/PickupActorInterface.Drop`
  (`PrimitiveComponent.SetSimulatePhysics` (`self.StaticMeshComponent`) true)
  (`self.K2_DetachFromActor` "KeepWorld" "KeepWorld" "KeepWorld")
  (set `self.IsHeld` false))

(fn `FireWeapon`
  (`|SpawnActorFromClass` "/Game/Weapons/Bullet.Bullet_C" (`KismetMathLibrary.MakeTransform` (`SceneComponent.K2_GetComponentLocation` (`self.Arrow`))) "Undefined" "OverrideRootScale" null null))

(fn `UserConstructionScript`)